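; BP_ShooterCharacter is a shooter character Blueprint with switchable first- and third-person cameras and an aim zoom.
; The ChangeCamera input toggles both camera components' active state.
; Zoom press and release share a FlipFlop that plays or reverses a timeline driving both FOVs, with first-person offset wider, and slightly lowers look sensitivity while zoomed.
; Disconnected sensitivity-factor and music nodes never run.
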(event `self.ReceiveBeginPlay`)

(event `InputAction|ChangeCamera`
  (params (Key :type "Key Structure"))
  ;[1 1 1] Switch Player Camera
  (:`Pressed`
    (`ActorComponent.ToggleActive` (`self.FPCamera`))
    (`ActorComponent.ToggleActive` (`self.TPCamera`))))

(event `InputAction|Zoom`
  (params (Key :type "Key Structure"))
  (bind _returnvalue (`GameplayStatics.GetPlayerController` 0))
  ;[1 1 1] Player Zoom
  (:`Pressed`
    (`/Engine/EditorBlueprintResources/StandardMacros.FlipFlop` :!label _label
      (:`A`
        (set `PlayerController.InputPitchScale` -0.95 _returnvalue)
        (set `PlayerController.InputYawScale` 0.95 _returnvalue)
        (bind (_direction _zoomintp) (`Timeline|ZoomInTP` :!via `PlayFromStart` :!label _label_2)
          (:`Update`
            (set `CameraComponent.FieldOfView` _zoomintp (`self.TPCamera`))
            (set `CameraComponent.FieldOfView` (+ _zoomintp 20.0) (`self.FPCamera`)))))
      (:`B`
        (set `PlayerController.InputPitchScale` -1.0 _returnvalue)
        (set `PlayerController.InputYawScale` 1.0 _returnvalue)
        (goto _label_2 :!via `ReverseFromEnd`))))
  (:`Released`
    (goto _label)))

(fn `UserConstructionScript`)